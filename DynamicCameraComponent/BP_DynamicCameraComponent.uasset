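; Vehicle camera component that adds speed-reactive framing and speed effects to its owning car.
; On BeginPlay it builds a configurable lag spring arm, attaches the tagged camera to it, and creates a Niagara speed effect on a follower arrow.
; Each tick, the follower tracks the arm's end, while forward speed shortens the arm, widens FOV and drives particle rate above a threshold.
; A look-at rotation for the arm exists but is disconnected.
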(event EventBeginPlay
  (bind _returnvalue (Components|GetOwner))
  (Utilities|FlowControl|Sequence
    (:then_0
      (Variables|Default|SetCar (Utilities|Array|Get(acopy) (Actor|GetComponentsbyTag _returnvalue "/Script/Engine.ActorComponent" "Car")))
      (Variables|Default|SetCamera (Utilities|Array|Get(acopy) (Actor|GetComponentsbyTag _returnvalue "/Script/Engine.CameraComponent" "Cam")))
      (Variables|Default|SetMovementComponent (Actor|GetComponentbyClass _returnvalue "/Script/ChaosVehicles.ChaosWheeledVehicleMovementComponent"))
      (bind _returnvalue_2 (Game|AddComponentbyClass _returnvalue "/Script/Engine.ArrowComponent" false))
      (Variables|Default|SetFollowCameraParent _returnvalue_2)
      (bind _returnvalue_3 (Game|AddComponentbyClass _returnvalue "/Script/Niagara.NiagaraComponent" false))
      (bind _output_get (Variables|Default|SetNiagara _returnvalue_3))
      (Transformation|AttachComponentToComponent _output_get (Variables|Default|GetFollowCameraParent) "None" "SnapToTarget" "SnapToTarget" "SnapToTarget" true)
      (Transformation|SetRelativeLocation _returnvalue_3 "230.000000,0.000000,0.000000" false false)
      (Class|NiagaraComponent|SetAsset _output_get "/Game/DynamicCameraComponent/SpeedFX.SpeedFX" true))
    (:then_1
      (bind _returnvalue_4 (Game|AddComponentbyClass _returnvalue "/Script/Engine.SpringArmComponent" false (Math|Transform|MakeTransform (Variables|Default|GetPivot) "0, 0, 0" "1.000000,1.000000,1.000000")))
      (Variables|Default|SetLagArm _returnvalue_4)
      (bind _returnvalue_5 (Game|AddComponentbyClass _returnvalue "/Script/Engine.ArrowComponent" false))
      (bind _output_get_2 (Variables|Default|SetLagParent _returnvalue_5))
      (Transformation|AttachComponentToComponent _output_get_2 (Variables|Default|GetLagArm) "None" "SnapToTarget" "SnapToTarget" "SnapToTarget" true)
      (Variables|/Script/Engine.SpringArmComponent|SetTargetArmLength (Variables|Default|GetLagArm) (Variables|Default|GetLagArmLength))
      (Variables|/Script/Engine.SpringArmComponent|SetbEnableCameraLag (Variables|Default|GetLagArm) (Variables|Default|GetCamera%20Lag))
      (Variables|/Script/Engine.SpringArmComponent|SetbEnableCameraRotationLag (Variables|Default|GetLagArm) (Variables|Default|GetCamera%20Rotation%20Lag))
      (Variables|/Script/Engine.SpringArmComponent|SetCameraLagSpeed (Variables|Default|GetLagArm) (Variables|Default|GetLagSpeed))
      (Variables|/Script/Engine.SpringArmComponent|SetCameraLagMaxDistance (Variables|Default|GetLagArm) (Variables|Default|GetLag%20Max%20Distance))
      (Variables|/Script/Engine.SpringArmComponent|SetCameraRotationLagSpeed (Variables|Default|GetLagArm) (Variables|Default|GetLagSpeedRotation))
      (Variables|/Script/Engine.SpringArmComponent|SetbDoCollisionTest (Variables|Default|GetLagArm) (Variables|Default|GetDo%20Collision%20Test)))
    (:then_2
      (Transformation|AttachComponentToComponent (Variables|Default|GetCamera) (Variables|Default|GetLagArm) "None" "SnapToTarget" "SnapToTarget" "SnapToTarget" true))))

(event EventTick
  (params (DeltaSeconds :type Float%20%28single-precision%29))
  (bind _movementcomponent (Variables|Default|GetMovementComponent))
  (bind _lagarm (Variables|Default|GetLagArm))
  (bind _lagparent (Variables|Default|GetLagParent))
  (bind _returnvalue (Vehicle|GetForwardSpeed _movementcomponent))
  (bind _returnvalue_2 (Transformation|GetWorldLocation _lagarm))
  (bind _returnvalue_3 (Transformation|GetWorldLocation _lagparent))
  (Transformation|SetWorldLocation (Variables|Default|GetFollowCameraParent) (Math|Vector|MakeVector (.x _returnvalue_3) (.y _returnvalue_3) (.z _returnvalue_3)) false false)
  (Variables|/Script/Engine.SpringArmComponent|SetTargetArmLength (Variables|Default|GetLagArm) (Math|Float|Lerp (Variables|Default|GetLagArmLength) 0.0 (/ _returnvalue 6666.0)))
  (Camera|SetFieldOfView (Variables|Default|GetCamera) (+ (* _returnvalue (Variables|Default|GetCamFOVmult)) 9e+01))
  (Variables|Default|SetSpeed (Math|Vector|Distance(Vector) _returnvalue_2 (Variables|Default|GetOldActorLocation)))
  (Effects|Components|ParticleSystem|SetFloatParameter (Variables|Default|GetNiagara) "Rate" (* (Math|Float|Clamp(Float) (- _returnvalue 1555.0) 0.0 999.0) 0.3))
  (Variables|Default|SetOldActorLocation _returnvalue_2))